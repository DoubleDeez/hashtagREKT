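; Behavior tree task for the Monster that sets its blackboard Destination, either stalking a player or wandering.
; It keeps its current victim while that player is alive and holding ShipParts, updating Destination to their location on each execution.
; Otherwise it picks a random qualifying player, falling back to a random point around the monster's spawn.
; It finishes successfully once Destination is written, leaving movement outside this task.
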(event EventReceiveExecute
  (params (OwnerActor :type Actor%20Object%20Reference))
  (bind _playerarray (Variables|Default|GetPlayerArray))
  (Variables|Default|SetOwner OwnerActor)
  (if (Variables|Default|GetHasAPlayer)
    ;[1 1 1] Check if victim died
    (if (Variables|/Game/Blueprints/Player/Player.Player_C|GetIsDead (Variables|Default|GetCurrentVictim))
      (Variables|Default|SetHasAPlayer false :!label _label)
      (Utilities|Array|Clear (Variables|Default|GetPlayerArray) :!label _label_2)
      ;[1 1 1] Create Array of Potential Victims
      (bind _outactors (Actor|GetAllActorsOfClass "/Game/Blueprints/Player/Player.Player_C"))
      (bind _array_element (Utilities|Array|ForEachLoopwithBreak _outactors)
        (:LoopBody
          (bind _asplayer (Utilities|Casting|CastToPlayer _array_element))
          (if (Math|Boolean|ANDBoolean (not (Variables|/Game/Blueprints/Player/Player.Player_C|GetIsDead _asplayer)) (Variables|/Game/Blueprints/Player/Player.Player_C|GetIsHoldingItem _asplayer) (== (Utilities|GetClass (Variables|/Game/Blueprints/Player/Player.Player_C|GetHeldItem _asplayer)) "/Game/Blueprints/Items/ShipParts.ShipParts_C"))
            (Utilities|Array|AddUnique (Variables|Default|GetPlayerArray) _asplayer)))
        (:Completed
          ;[1 1 1] Wander if no victims
          (if (> (Utilities|Array|Length (Variables|Default|GetPlayerArray)) 0)
            ;[0.535 0 0.03824] Pick random victim and stalk
            (Variables|Default|SetCurrentVictim (Utilities|Array|Get(acopy) _playerarray (Math|Random|RandomIntegerinRange 0 (- (Utilities|Array|Length _playerarray) 1))))
            (Variables|Default|SetHasAPlayer true)
            (AI|BehaviorTree|SetBlackboardValueasVector (Variables|Default|GetDestination) (Transformation|GetActorLocation (Variables|Default|GetCurrentVictim)))
            (else
              (bind _asmonster_controller (Utilities|Casting|CastToMonsterController (Variables|Default|GetOwner)))
              (bind _asmonster (Utilities|Casting|CastToMonster (Pawn|GetControlledPawn _asmonster_controller)))
              (AI|BehaviorTree|SetBlackboardValueasVector (Variables|Default|GetDestination) (Class|NavigationSystem|GetRandomPointinRadius (Variables|/Game/Blueprints/Monster/Monster.Monster_C|GetSpawnLocation _asmonster) 1.2e+03))))
          (AI|BehaviorTree|FinishExecute true :!label _label_3)))
      (else
        ;[1 1 1] Player no longer has ship parts
        (if (and (Variables|/Game/Blueprints/Player/Player.Player_C|GetIsHoldingItem (Variables|Default|GetCurrentVictim)) (== (Utilities|GetClass (Variables|/Game/Blueprints/Player/Player.Player_C|GetHeldItem (Variables|Default|GetCurrentVictim))) "/Game/Blueprints/Items/ShipParts.ShipParts_C"))
          ;[1 1 1] Stalk victim
          (AI|BehaviorTree|SetBlackboardValueasVector (Variables|Default|GetDestination) (Transformation|GetActorLocation (Variables|Default|GetCurrentVictim)))
          (goto _label_3)
          (else
            (goto _label)))))
    (else
      (goto _label_2))))