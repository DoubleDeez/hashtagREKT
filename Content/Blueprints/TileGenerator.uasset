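; TileGenerator builds a tile map at BeginPlay by spawning a rotated tile actor for each TileMap entry.
; Each value selects a class, 0 for dirt and 255 for grass.
; The array index is split into column and row by TileLength.
; CalculateLocation holds a grid-position vector scaled by TileSize, but that node is unconnected, so the computed position goes unused.
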(event EventBeginPlay
  (for (_array_element _array_index) (Variables|Default|GetTileMap)
    (CallFunction|SetColandRowfromIndex _array_index)
    (bind _sprite_val (CallFunction|TileClassfromMap _array_element))
    (Game|SpawnActorfromClass _sprite_val (Math|Transform|MakeTransform (Utilities|CalculateLocation) "0,90.000000,-90.000000") true 0)))

(fn ConstructionScript)

(fn TileClassfromMap
  (params (TileMapValue :type Integer))
  (LocalVariables|SetTileMapVal TileMapValue)
  (if (== (LocalVariables|GetTileMapVal) 0)
    (LocalVariables|SetNewSprite "/Game/Blueprints/Tile_Dirt.Tile_Dirt_C")
    (elif (== (LocalVariables|GetTileMapVal) 255)
      (LocalVariables|SetNewSprite "/Game/Blueprints/Tile_Grass.Tile_Grass_C")))
  (return (LocalVariables|GetNewSprite)))

(fn SetColandRowfromIndex
  (params (Index :type Integer))
  (bind _tilelength (Variables|Default|GetTileLength))
  (Variables|Default|SetColumn (/ Index _tilelength))
  (Variables|Default|SetRow (Math|Integer|%(Integer) Index _tilelength)))