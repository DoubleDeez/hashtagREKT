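; Player character Blueprint with joystick movement, a fixed-angle camera and item pickup.
; Forward and Right axes drive movement along fixed world directions, turn the mesh toward the input vector and feed a speed ratio to Player_Anim.
; A self-repeating BeginPlay delay loop keeps reapplying the camera's world rotation.
; The top gamepad face button picks up the last Item overlapping the capsule unless one is already held.
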(event Custom|RepeatBeginPlay
  ;[1 1 1] Fixed camera
  (Transformation|SetWorldRotation "-50.000000,-180.000000, 0" false)
  (Utilities|FlowControl|Delay 0.1)
  (CallFunction|RepeatBeginPlay))

(event EventBeginPlay
  ;[1 1 1] Fixed camera
  (Transformation|SetWorldRotation "-50.000000,-180.000000, 0" false)
  (Utilities|FlowControl|Delay 0.1)
  (CallFunction|RepeatBeginPlay))

(event Input|AxisEvents|InputAxisForward
  (params (AxisValue :type Float%20%28single-precision%29))
  (bind _xinput (Variables|Default|GetXInput))
  ;[1 1 1] Character Movement with Left Joystick
  (Variables|Default|SetYInput AxisValue)
  (Pawn|Input|AddMovementInput "-1.000000, 0, 0" AxisValue false)
  ;[1 1 1] Set direction of mesh
  (if (Math|Boolean|ORBoolean (> _xinput 0.01) (< _xinput -0.01) (> (Variables|Default|GetYInput) 0.01) (< (Variables|Default|GetYInput) -0.01))
    (Transformation|SetWorldRotation (Math|Rotator|MakeRotfromX (Math|Vector|Normalize (Math|Vector|MakeVector _xinput (Variables|Default|GetYInput) 0.0))) false)))

(event Input|AxisEvents|InputAxisRight
  (params (AxisValue :type Float%20%28single-precision%29))
  ;[1 1 1] Character Movement with Left Joystick
  (Variables|Default|SetXInput (* AxisValue -1.0))
  (Pawn|Input|AddMovementInput "0,-1.000000, 0" AxisValue false)
  ;[1 1 1] Set speed ratio var for animation
  (bind _asplayer_anim (Utilities|Casting|CastToPlayer_Anim (Components|SkeletalMesh|GetAnimInstance (Variables|Character|GetMesh))))
  (Variables|/Game/Blueprints/Player/Player_Anim.Player_Anim_C|SetSpeed _asplayer_anim (/ (Math|Vector|VectorLength (Transformation|GetVelocity)) (Class|MovementComponent|GetMaxSpeed))))

(event Input|GamepadEvents|GamepadFaceButtonTop
  (bind _capsulecomponent (Variables|Collision|GetCapsuleComponent))
  (bind _overlappingactors (Collision|GetOverlappingActors _capsulecomponent "/Game/Blueprints/Items/Item.Item_C" :!class /Script/Engine.PrimitiveComponent))
  ;[1 1 1] Item Pickup
  (:Pressed
    (if (and (!= (Utilities|Array|Length _overlappingactors) 0) (not (Variables|Default|GetIsHoldingItem)))
      (bind _asitem (Utilities|Casting|CastToItem (Utilities|Array|Get(acopy) _overlappingactors (Utilities|Array|LastIndex _overlappingactors))))
      (Default|PickupItem _asitem))))

(fn ConstructionScript)