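; Item is a world pickup Blueprint that shows a text hint when the player is near and can be picked up and dropped.
; TriggerVolume overlaps toggle the PickMeUp hint and the actor's player input while the item is not picked up.
; PickupItem hides the hint, sets IsPickedUp and switches Mesh collision to overlap.
; DropItem shows mesh and hint, moves the components beside a given location and restores blocking collision.
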(event OnComponentBeginOverlap(TriggerVolume)
  (params (OtherActor :type Actor%20Object%20Reference) (OtherComp :type Primitive%20Component%20Object%20Reference) (OtherBodyIndex :type Integer) (bFromSweep :type Boolean) (SweepResult :type Hit%20Result%20Structure%20%28by%20ref%29))
  ;[1 1 1] Display text hint to pick up item when near
  (if (and (== OtherActor (Game|Player|GetPlayerPawn 0)) (not (Variables|Default|GetIsPickedUp)))
    (Input|EnableInput (Game|GetPlayerController 0))
    (Rendering|SetVisibility (Variables|Default|GetPickMeUp) true false)))

(event OnComponentEndOverlap(TriggerVolume)
  (params (OtherActor :type Actor%20Object%20Reference) (OtherComp :type Primitive%20Component%20Object%20Reference) (OtherBodyIndex :type Integer))
  ;[1 1 1] Display text hint to pick up item when near
  (if (and (== (stale OnComponentBeginOverlap(TriggerVolume) OtherActor) (Game|Player|GetPlayerPawn 0)) (not (Variables|Default|GetIsPickedUp)))
    (Input|DisableInput (Game|GetPlayerController 0))
    (Rendering|SetVisibility (Variables|Default|GetPickMeUp) false false)))

(event EventBeginPlay
  (Rendering|SetVisibility (Variables|Default|GetPickMeUp) false false))

(fn ConstructionScript
  (Rendering|SetVisibility (Variables|Default|GetPickMeUp) false false)
  (Variables|Default|SetIsPickedUp false))

(fn PickupItem
  (Rendering|SetVisibility (Variables|Default|GetPickMeUp) false false)
  (Variables|Default|SetIsPickedUp true)
  (Collision|SetCollisionResponsetoAllChannels (Variables|Default|GetMesh) "ECR_Overlap"))

(fn DropItem
  (params (Location :type Vector))
  (bind (_x _y _z) (Math|Vector|BreakVector Location))
  (bind _mesh (Variables|Default|GetMesh))
  (Rendering|SetVisibility _mesh true false)
  (Transformation|SetWorldLocation _mesh (Math|Vector|MakeVector (+ _x 5e+01) (+ _y 5e+01) _z) false)
  (Variables|Default|SetIsPickedUp false)
  (Collision|SetCollisionResponsetoAllChannels _mesh "ECR_Block"))