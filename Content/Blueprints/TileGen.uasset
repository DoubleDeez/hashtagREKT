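; TileGen procedurally builds a tile island surrounded by water on BeginPlay, spawning actors only on the authority.
; An IslandSize-driven grid gets random grass or dirt from RandomTile, whose returned value selects the scatter: rocks on grass, bushes or trees on dirt, via chained low-chance rolls.
; Further loops add sand and shallow water bands along both Y edges, with deep water beyond them and along both X sides.
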(event EventBeginPlay
  (bind _returnvalue (Math|Random|RandomIntegerinRange 0 100))
  (bind _returnvalue_2 (Math|Random|RandomIntegerinRange 0 100))
  (bind _islandsize (Variables|Default|GetIslandSize))
  (bind _islandsize_2 (Variables|Default|GetIslandSize))
  (bind _islandsize_3 (Variables|Default|GetIslandSize))
  (bind _islandsize_4 (Variables|Default|GetIslandSize))
  (bind _returnvalue_3 (/ _islandsize_3 2))
  (bind _returnvalue_4 (- _islandsize_4 1))
  (bind _returnvalue_5 (/ _islandsize 4))
  (bind _returnvalue_6 (/ _islandsize_2 8))
  (bind _returnvalue_7 (/ _islandsize_3 4))
  (Networking|SwitchHasAuthority
    (:Authority
      (for _index (range 1 _returnvalue_4)
        (for _index_2 (range 1 _returnvalue_4)
          (bind (_tile _value) (CallFunction|RandomTile))
          (Game|SpawnActorfromClass _tile (Math|Transform|MakeTransform (Math|Vector|MakeVector (Math|Conversions|ToFloat(Integer) (* _index 100)) (Math|Conversions|ToFloat(Integer) (* _index_2 100)) 0.0) "0,90.000000,-90.000000") true 0)
          (if (== _value 0)
            (if (< _returnvalue_2 5)
              (Game|SpawnActorfromClass "/Game/Blueprints/Rock_01.Rock_01_C" (Math|Transform|MakeTransform (Math|Vector|MakeVector (Math|Conversions|ToFloat(Integer) (* _index 100)) (Math|Conversions|ToFloat(Integer) (* _index_2 100)) 0.0) "0,270.000000, 0") true 0)
              (elif (< _returnvalue_2 5)
                (Game|SpawnActorfromClass "/Game/Blueprints/Rock_02.Rock_02_C" (Math|Transform|MakeTransform (Math|Vector|MakeVector (Math|Conversions|ToFloat(Integer) (* _index 100)) (Math|Conversions|ToFloat(Integer) (* _index_2 100)) 0.0) "0,270.000000, 0") true 0)
                (elif (< _returnvalue_2 5)
                  (Game|SpawnActorfromClass "/Game/Blueprints/Rock_03.Rock_03_C" (Math|Transform|MakeTransform (Math|Vector|MakeVector (Math|Conversions|ToFloat(Integer) (* _index 100)) (Math|Conversions|ToFloat(Integer) (* _index_2 100)) 0.0) "0,270.000000, 0") true 0)
                  (elif (< _returnvalue_2 5)
                    (Game|SpawnActorfromClass "/Game/Blueprints/Rock_04.Rock_04_C" (Math|Transform|MakeTransform (Math|Vector|MakeVector (Math|Conversions|ToFloat(Integer) (* _index 100)) (Math|Conversions|ToFloat(Integer) (* _index_2 100)) 0.0) "0,270.000000, 0") true 0)))))
            (elif (== _value 1)
              (if (< _returnvalue 5)
                (Game|SpawnActorfromClass "/Game/Blueprints/Bush_01.Bush_01_C" (Math|Transform|MakeTransform (Math|Vector|MakeVector (Math|Conversions|ToFloat(Integer) (* _index 100)) (Math|Conversions|ToFloat(Integer) (* _index_2 100)) 0.0) "0,270.000000, 0") true 0)
                (elif (< _returnvalue 5)
                  (Game|SpawnActorfromClass "/Game/Blueprints/Bush_02.Bush_02_C" (Math|Transform|MakeTransform (Math|Vector|MakeVector (Math|Conversions|ToFloat(Integer) (* _index 100)) (Math|Conversions|ToFloat(Integer) (* _index_2 100)) 0.0) "0,270.000000, 0") true 0)
                  (elif (< _returnvalue 5)
                    (Game|SpawnActorfromClass "/Game/Blueprints/Tree_01.Tree_01_C" (Math|Transform|MakeTransform (Math|Vector|MakeVector (Math|Conversions|ToFloat(Integer) (* _index 100)) (Math|Conversions|ToFloat(Integer) (* _index_2 100)) 0.0) "0,270.000000, 0") true 0)
                    (elif (< _returnvalue 5)
                      (Game|SpawnActorfromClass "/Game/Blueprints/Tree_02.Tree_02_C" (Math|Transform|MakeTransform (Math|Vector|MakeVector (Math|Conversions|ToFloat(Integer) (* _index 100)) (Math|Conversions|ToFloat(Integer) (* _index_2 100)) 0.0) "0,270.000000, 0") true 0)))))))))
      (for _index_3 (range 1 _returnvalue_4)
        (for _index_4 (range 0 (- (/ _islandsize 8) 1))
          (Game|SpawnActorfromClass "/Game/Blueprints/Tiles/Tile_Sand.Tile_Sand_C" (Math|Transform|MakeTransform (Math|Vector|MakeVector (Math|Conversions|ToFloat(Integer) (* _index_3 100)) (Math|Conversions|ToFloat(Integer) (* _index_4 -100)) 0.0) "0,90.000000,-90.000000") true 0)
          (Game|SpawnActorfromClass "/Game/Blueprints/Tiles/Tile_Sand.Tile_Sand_C" (Math|Transform|MakeTransform (Math|Vector|MakeVector (Math|Conversions|ToFloat(Integer) (* _index_3 100)) (Math|Conversions|ToFloat(Integer) (* (+ _index_4 _islandsize) 100)) 0.0) "0,90.000000,-90.000000") true 0)))
      (for _index_5 (range 0 _returnvalue_5)
        (for _index_6 (range (* _returnvalue_5 -2) (+ _returnvalue_5 _islandsize _returnvalue_5))
          (Game|SpawnActorfromClass "/Game/Blueprints/Tiles/Tile_DeepWater.Tile_DeepWater_C" (Math|Transform|MakeTransform (Math|Vector|MakeVector (Math|Conversions|ToFloat(Integer) (* _index_5 -100)) (Math|Conversions|ToFloat(Integer) (* _index_6 100)) 0.0) "0,90.000000,-90.000000") true 0)
          (Game|SpawnActorfromClass "/Game/Blueprints/Tiles/Tile_DeepWater.Tile_DeepWater_C" (Math|Transform|MakeTransform (Math|Vector|MakeVector (Math|Conversions|ToFloat(Integer) (* (+ _index_5 _islandsize) 100)) (Math|Conversions|ToFloat(Integer) (* _index_6 100)) 0.0) "0,90.000000,-90.000000") true 0)))
      (for _index_7 (range 1 (- _islandsize_2 1))
        (for _index_8 (range 0 (/ _islandsize_2 2))
          (Game|SpawnActorfromClass "/Game/Blueprints/Tiles/Tile_Water.Tile_Water_C" (Math|Transform|MakeTransform (Math|Vector|MakeVector (Math|Conversions|ToFloat(Integer) (* _index_7 100)) (Math|Conversions|ToFloat(Integer) (* (+ _index_8 _returnvalue_6) -100)) 0.0) "0,90.000000,-90.000000") true 0)
          (Game|SpawnActorfromClass "/Game/Blueprints/Tiles/Tile_Water.Tile_Water_C" (Math|Transform|MakeTransform (Math|Vector|MakeVector (Math|Conversions|ToFloat(Integer) (* _index_7 100)) (Math|Conversions|ToFloat(Integer) (* (+ _index_8 _islandsize_2 _returnvalue_6) 100)) 0.0) "0,90.000000,-90.000000") true 0)))
      (for _index_9 (range (* _returnvalue_7 -1) (+ _islandsize_3 _returnvalue_7))
        (for _index_10 (range 0 _returnvalue_3)
          (Game|SpawnActorfromClass "/Game/Blueprints/Tiles/Tile_DeepWater.Tile_DeepWater_C" (Math|Transform|MakeTransform (Math|Vector|MakeVector (Math|Conversions|ToFloat(Integer) (* _index_9 100)) (Math|Conversions|ToFloat(Integer) (* (+ _index_10 _returnvalue_3) -100)) 0.0) "0,90.000000,-90.000000") true 0)
          (Game|SpawnActorfromClass "/Game/Blueprints/Tiles/Tile_DeepWater.Tile_DeepWater_C" (Math|Transform|MakeTransform (Math|Vector|MakeVector (Math|Conversions|ToFloat(Integer) (* _index_9 100)) (Math|Conversions|ToFloat(Integer) (* (+ _index_10 _returnvalue_3 _islandsize_3) 100)) 0.0) "0,90.000000,-90.000000") true 0))))))

(fn ConstructionScript)

(fn RandomTile
  (LocalVariables|SetRandomValue (Math|Random|RandomIntegerinRange 0 1))
  (switch int (LocalVariables|GetRandomValue)
    (:0
      (LocalVariables|SetTileClass "/Game/Blueprints/Tiles/Tile_Grass.Tile_Grass_C"))
    (:1
      (LocalVariables|SetTileClass "/Game/Blueprints/Tiles/Tile_Dirt.Tile_Dirt_C")))
  (return (LocalVariables|GetTileClass) (LocalVariables|GetRandomValue)))