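; Repairable boat that players rebuild from six ShipParts and board while holding an Oar.
; Each tick it counts overlapping parts not being carried, shows progress, and at six swaps to the fixed sprite and marks itself built.
; Once built, it hides parts in PartsCollider, shows a boarding prompt and eases toward a fixed destination, with or without passengers.
; Embark01 registers overlapping Oar holders, whom Tick pins to the boat's location.
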(event Custom|Embark01
  (if (Variables|Default|GetShipIsBuilt)
    (for _array_element (Collision|GetOverlappingActors (Variables|Default|GetPartsCollider) "/Game/Blueprints/Player/Player.Player_C" :!class /Script/Engine.PrimitiveComponent)
      (bind _asplayer (Utilities|Casting|CastToPlayer _array_element))
      (if (== (Utilities|GetClass (Variables|/Game/Blueprints/Player/Player.Player_C|GetHeldItem _asplayer)) "/Game/Blueprints/Items/Oar.Oar_C")
        (Utilities|Array|Add (Variables|Default|GetPlayersInBoat) _asplayer)))))

(event EventTick
  (params (DeltaSeconds :type Float%20%28single-precision%29))
  (Variables|Default|SetDelta DeltaSeconds)
  (for _array_element (Variables|Default|GetPlayersInBoat)
    (Transformation|SetActorLocation _array_element (Transformation|GetActorLocation) false))
  (if (Variables|Default|GetShipIsBuilt)
    (for _array_element_2 (Collision|GetOverlappingActors (Variables|Default|GetPartsCollider) "/Game/Blueprints/Items/ShipParts.ShipParts_C" :!class /Script/Engine.PrimitiveComponent)
      (bind _asship_parts (Utilities|Casting|CastToShipParts _array_element_2))
      (Rendering|SetActorHiddenInGame _asship_parts true)
      (Collision|SetCollisionEnabled _asship_parts "NoCollision"))
    (Rendering|Components|TextRender|SetText (Variables|Default|GetTextRender1) "Grab an Ore and Press 'A' to embark")
    (Rendering|Components|Sprite|SetSprite (Variables|Default|GetPaperSprite1) "/Game/Sprites/Boat_Fixed.Boat_Fixed")
    (Transformation|SetActorLocation (Math|Vector|Lerp(Vector) (Transformation|GetActorLocation) "700.000000,5000.000000,38.000000" (* (Variables|Default|GetDelta) 0.05)) false)
    (else
      (Variables|Default|SetPartsCount 0)
      (for _array_element_3 (Collision|GetOverlappingActors "/Game/Blueprints/Items/ShipParts.ShipParts_C" :!class /Script/Engine.PrimitiveComponent)
        (bind _asship_parts_2 (Utilities|Casting|CastToShipParts _array_element_3))
        (if (not (Variables|/Game/Blueprints/Items/Item.Item_C|GetIsPickedUp _asship_parts_2))
          (Variables|Default|SetPartsCount (+ (Variables|Default|GetPartsCount) 1))))
      (Rendering|Components|TextRender|SetText (Variables|Default|GetTextRender1) (Utilities|String|Append (Utilities|String|Append (Variables|Default|GetPartsString) (Utilities|String|ToString(Integer) (Variables|Default|GetPartsCount))) "/6"))
      (if (== (Variables|Default|GetPartsCount) 6)
        (Rendering|Components|TextRender|SetText (Variables|Default|GetTextRender1) "")
        (Rendering|Components|Sprite|SetSprite (Variables|Default|GetPaperSprite1) "/Game/Sprites/Boat_Fixed.Boat_Fixed")
        (Variables|Default|SetShipIsBuilt true)
        (for _array_element_4 (Collision|GetOverlappingActors (Variables|Default|GetPartsCollider) "/Game/Blueprints/Items/ShipParts.ShipParts_C" :!class /Script/Engine.PrimitiveComponent)
          (bind _asship_parts_3 (Utilities|Casting|CastToShipParts _array_element_4))
          (Default|PickupItem _asship_parts_3))))))

(fn ConstructionScript)